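; Scientist actor Blueprint that randomly switches a Paper2D character between walk, run and two surprised flipbook animations.
; Tick accumulates delta time and, whenever the timer passes two seconds, resets it and rolls a random index.
; The AnimStateMachine function is a simple Select mapping that index to a flipbook for the FLABGUYwork component.
; Debug prints show the timer and a separately rolled random number.
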(event EventBeginPlay
  (Variables|Default|SetCountdown 0.0))

(event Collision|EventActorBeginOverlap
  (params (OtherActor :type Actor%20Object%20Reference)))

(event EventTick
  (params (DeltaSeconds :type Float%20%28single-precision%29))
  (bind _returnvalue (Math|Random|RandomIntegerinRange 0 3))
  (if (> (Variables|Default|GetCountdown) 2.0)
    (Variables|Default|SetCountdown 0.0)
    (Development|PrintText (Utilities|Text|ToText(Integer) _returnvalue))
    (bind _output_get (Variables|Default|SetRandInt _returnvalue))
    (bind _newparam (CallFunction|AnimStateMachine _output_get))
    (Sprite|SetFlipbook (Variables|Default|GetF_LABGUYwork) _newparam)
    (else
      (bind _output_get_2 (Variables|Default|SetCountdown (+ DeltaSeconds (Variables|Default|GetCountdown))))
      (Development|PrintText (Utilities|Text|ToText(Float) _output_get_2 "HalfToEven")))))

(fn ConstructionScript)

(fn AnimStateMachine
  (params (RandInt :type Integer))
  (return (Utilities|Select :Index RandInt :Option%200 (Variables|Default|GetWalkFlipBook) :Option%201 (Variables|Default|GetRunFlipBook) :Option%202 (Variables|Default|GetSuprised2FlipBook) :Option%203 (Variables|Default|GetSuprised1FlipBook))))