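; BP_Plant is a 2D Paper2D plant actor that grows on demand and becomes solid or interactive after a timed delay.
; TogglePlantCreation resets the timer, flags growth and starts the growth flipbook.
; Tick accumulates time and, once growth is flagged and the delay has elapsed, fires PlantActivation a single time.
; Activation freezes the flipbook, reveals the PaperSprite and enables collision on three boxes.
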(event EventBeginPlay)

(event Collision|EventActorBeginOverlap
  (params (OtherActor :type Actor%20Object%20Reference)))

(event EventTick
  (params (DeltaSeconds :type Float%20%28single-precision%29))
  (Variables|Default|SetTimeWaiting (+ DeltaSeconds (Variables|Default|GetTimeWaiting)))
  (if (Math|Boolean|ANDBoolean (Variables|Default|GetPlantGrowth) (not (Variables|Default|GetPlantActivated)) (>= (Variables|Default|GetTimeWaiting) (Variables|Default|GetTimeWaitingToSwitch)))
    (Development|PrintString "tayo")
    (Variables|Default|SetPlantActivated true)
    (CallFunction|PlantActivation)))

(fn ConstructionScript)

(fn TogglePlantCreation
  (Variables|Default|SetTimeWaiting 0.0)
  (Variables|Default|SetPlantGrowth true)
  (Sprite|SetFlipbook (Variables|Default|GetF_Plant) "/Game/Prune/F_PLANT.F_PLANT")
  (Components|Timeline|SetPlayRate (Variables|Default|GetF_Plant) 1.0)
  (return))

(fn PlantActivation
  (Rendering|SetVisibility (Variables|Default|GetPaperSprite) true false)
  (Collision|SetCollisionEnabled (Variables|Default|GetBox2) "QueryAndPhysics")
  (Collision|SetCollisionEnabled (Variables|Default|GetBox1) "QueryAndPhysics")
  (Collision|SetCollisionEnabled (Variables|Default|GetBox) "QueryAndPhysics")
  (Components|Timeline|SetPlayRate (Variables|Default|GetF_Plant) 0.0)
  (return))