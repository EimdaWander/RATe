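; Player pawn for a 2D flipbook side-scroller, handling Enhanced Input movement, jumping and the pause menu.
; Movement follows control-yaw forward, and each Tick mirrors the sprite by X velocity sign through negative scale.
; A small state function picks the Idle, Run or Jump flipbook from velocity and jump-input state, not airborne status.
; The pause input toggles the menu widget, game pause, input mode and cursor.
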(event Custom|UpdateAnimation
  (bind _output_get (Variables|Default|SetIsMoving (> (Math|Vector|VectorLength (Transformation|GetVelocity)) 0.0)))
  (bind _returnvalue (CallFunction|AnimStateMachine _output_get (Variables|Default|GetIsJumping)))
  (Sprite|SetFlipbook (Variables|Default|GetF_RATidle) _returnvalue))

(event Input|EnhancedActionEvents|EnhancedInputActionIA_Jump
  (params (ActionValue :type Float%20%28double-precision%29) (ElapsedSeconds :type Float%20%28double-precision%29) (TriggeredSeconds :type Float%20%28double-precision%29) (InputAction :type Input%20Action%20Object%20Reference :default "/Game/Celeste/Input/IA_Jump.IA_Jump"))
  (:Triggered
    (Character|Jump)
    (Variables|Default|SetIsJumping true))
  (:Completed
    (Character|StopJumping)
    (Variables|Default|SetIsJumping false)))

(event Input|EnhancedActionEvents|EnhancedInputActionIA_Movement
  (params (ActionValue :type Float%20%28double-precision%29) (ElapsedSeconds :type Float%20%28double-precision%29) (TriggeredSeconds :type Float%20%28double-precision%29) (InputAction :type Input%20Action%20Object%20Reference :default "/Game/Celeste/Input/IA_Movement.IA_Movement"))
  (:Triggered
    (Pawn|Input|AddMovementInput (Math|Vector|GetForwardVector (Math|Rotator|MakeRotator 0.0 0.0 (.yaw (Pawn|GetControlRotation :!class /Script/Engine.Pawn)))) ActionValue false)))

(event Input|EnhancedActionEvents|EnhancedInputActionIA_PauseGame
  (params (ActionValue :type Boolean) (ElapsedSeconds :type Float%20%28double-precision%29) (TriggeredSeconds :type Float%20%28double-precision%29) (InputAction :type Input%20Action%20Object%20Reference :default "/Game/Celeste/Input/IA_PauseGame.IA_PauseGame"))
  (bind _returnvalue (Game|GetPlayerController 0))
  ;[1 1 1] Input PauseMenu et ControllerSourisButton
  (:Started
    (if (not (Variables|Default|GetisPauseMenuOpened))
      (Variables|Default|SetisPauseMenuOpened true)
      (bind _returnvalue_2 (Game|ConstructObjectfromClass _returnvalue "/Game/Celeste/WB_PauseMenu.WB_PauseMenu_C"))
      (bind _output_get (Variables|Default|SetPauseMenuWidget _returnvalue_2))
      (UserInterface|Viewport|AddtoViewport _output_get 0)
      (Input|SetInputModeGameandUI _returnvalue (Variables|Default|GetPauseMenuWidget) "DoNotLock" true false)
      (Variables|/Script/Engine.PlayerController|SetbShowMouseCursor (Game|GetPlayerController 0) true)
      (Game|SetGamePaused true)
      (else
        (Variables|Default|SetisPauseMenuOpened false)
        (Widget|RemovefromParent (Variables|Default|GetPauseMenuWidget))
        (Game|SetGamePaused false)
        (Input|SetInputModeGameOnly _returnvalue false)
        (Variables|/Script/Engine.PlayerController|SetbShowMouseCursor (Game|GetPlayerController 0) false)))))

(event EventBeginPlay
  (Input|AddMappingContext (PlayerController|LocalPlayerSubsystems|GetEnhancedInputLocalPlayerSubsystem (Game|GetPlayerController 0)) "/Game/Celeste/Input/IMC_BaseInput.IMC_BaseInput" 0 "(bIgnoreAllPressedKeysUntilRelease=True,bForceImmediately=False)"))

(event Collision|EventActorBeginOverlap
  (params (OtherActor :type Actor%20Object%20Reference)))

(event EventTick
  (params (DeltaSeconds :type Float%20%28single-precision%29))
  (CallFunction|UpdateAnimation)
  (if (>= (.x (Transformation|GetVelocity)) 0.0)
    (Transformation|SetRelativeScale3D (Variables|Default|GetF_RATidle) "-0.228609,0.228609,0.228609")
    (else
      (Transformation|SetRelativeScale3D (Variables|Default|GetF_RATidle) "0.228609,0.228609,0.228609"))))

(fn ConstructionScript)

(fn AnimStateMachine
  (params (IsMoving? :type Boolean) (IsJumping? :type Boolean))
  (if IsMoving?
    (if IsJumping?
      (Variables|Default|SetAnimState "NewEnumerator2" :!label _label)
      (else
        (Variables|Default|SetAnimState "NewEnumerator1")))
    (elif IsJumping?
      (goto _label)
      (else
        (Variables|Default|SetAnimState "NewEnumerator0"))))
  (return (Utilities|Select :Index (Variables|Default|GetAnimState) :NewEnumerator0 (Variables|Animations|GetIdleFlipBook) :NewEnumerator1 (Variables|Animations|GetMoveFlipBook) :NewEnumerator2 (Variables|Animations|GetJumpFlipBook))))